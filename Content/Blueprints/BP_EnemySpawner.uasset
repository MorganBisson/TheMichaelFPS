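; BP_EnemySpawner is a destructible spawner that periodically spawns AI enemies at random navigable points around itself.
; A looping timer starts on BeginPlay or, if configured, when the player overlaps SpawnArea.
; It destroys itself with a hit effect when its enemy count runs out or damage depletes its protection points.
; It creates a dynamic material instance, but the parameter updates are unconnected TODO stubs.
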(event OnComponentBeginOverlap(SpawnArea)
  (params (OverlappedComponent :type Primitive%20Component%20Object%20Reference) (OtherActor :type Actor%20Object%20Reference) (OtherComp :type Primitive%20Component%20Object%20Reference) (OtherBodyIndex :type Integer) (bFromSweep :type Boolean) (SweepResult :type Hit%20Result%20Structure%20%28by%20ref%29))
  (if (and (== OtherActor (Game|Player|GetPlayerPawn 0)) (Variables|Default|GetOnlySpawnEnemiesWhenPlayerOverlapsTheArea))
    (Utilities|Time|SetTimerbyEvent (delegate Custom|SpawnEnemy) (Variables|Default|GetDurationBetweenSpawn) true)))

(event Custom|SpawnEnemy
  (AI|SpawnAIFromClass (Variables|Default|GetEnemyClass) 0 (+ (.RandomLocation (Class|NavigationSystemV1|GetRandomPointinNavigableRadius (Transformation|GetActorLocation) (Variables|Default|GetSpawnRadius) 0 0)) "0, 0,100.000000") "0, 0, 0" true 0)
  (bind _result (Math|Integer|DecrementInt (Variables|Default|GetEnemiesToSpawn))
    (:%20%20
      (if (<= _result 0)
        ;[1 1 1] Damages
        ;;[1 0.008883 0] Destroy
        (Niagara|SpawnSystematLocation "/Game/ThirdParty/Stylized_VFX_StPack/Particles/P_Hits.P_Hits" (Transformation|GetWorldLocation (Variables|Default|GetStaticMesh)))
        (Actor|DestroyActor)))))

(event EventBeginPlay
  (bind _staticmesh (Variables|Default|GetStaticMesh))
  ;[1 1 1] Init data
  (Variables|Default|SetCurrentProtectionPoints (Variables|Default|GetDefaultProtectionPoints))
  (bind _returnvalue (Rendering|Material|CreateDynamicMaterialInstance _staticmesh 0 (Rendering|Material|GetMaterial _staticmesh 0) "None" :!class /Script/Engine.PrimitiveComponent))
  (Variables|Default|SetMI_EnemySpawner _returnvalue)
  (if (not (Variables|Default|GetOnlySpawnEnemiesWhenPlayerOverlapsTheArea))
    (Utilities|Time|SetTimerbyEvent (delegate Custom|SpawnEnemy) (Variables|Default|GetDurationBetweenSpawn) true)))

(event Game|Damage|EventAnyDamage
  (params (Damage :type Float%20%28single-precision%29) (DamageType :type Damage%20Type%20Object%20Reference) (InstigatedBy :type Controller%20Object%20Reference) (DamageCauser :type Actor%20Object%20Reference))
  ;[1 1 1] Damages
  (bind _output_get (Variables|Default|SetCurrentProtectionPoints (- (Variables|Default|GetCurrentProtectionPoints) Damage)))
  (if (<= _output_get 0.0)
    ;;[1 0.008883 0] Destroy
    (Niagara|SpawnSystematLocation "/Game/ThirdParty/Stylized_VFX_StPack/Particles/P_Hits.P_Hits" (Transformation|GetWorldLocation (Variables|Default|GetStaticMesh)))
    (Actor|DestroyActor)))

(fn ConstructionScript)