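; BP_Cactus_Proj is the cactus enemy's projectile, a physics sphere launched on BeginPlay by a velocity-change impulse, with optional gravity.
; The construction script picks projectile and explosion effects by Level; color, size and per-tick position feed in as User parameters.
; Hits on actors not tagged Enemy apply damage each time.
; The first such hit also stops physics and collision, triggers the explosion and destroys the actor after delays.
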(event OnComponentHit(Sphere)
  (params (HitComponent :type Primitive%20Component%20Object%20Reference) (OtherActor :type Actor%20Object%20Reference) (OtherComp :type Primitive%20Component%20Object%20Reference) (NormalImpulse :type Vector :default "0, 0, 0") (Hit :type Hit%20Result%20Structure%20%28by%20ref%29))
  (bind _sphere (Variables|Default|GetSphere))
  ;[1 1 1] Explode if collision
  (if (not (Actor|ActorHasTag (.hitactor Hit) "Enemy"))
    (Utilities|FlowControl|Sequence
      (:then_0
        (Game|Damage|ApplyDamage (.hitactor Hit) (Variables|Default|GetDamageOnPlayer) 0 self))
      (:then_1
        (Utilities|FlowControl|DoOnce false
          (:Completed
            (Physics|SetSimulatePhysics _sphere false)
            (Collision|SetCollisionEnabled _sphere "NoCollision")
            (Components|Activation|Activate (Variables|Default|GetExplosion) true)
            (Utilities|FlowControl|Delay 0.5)
            (Components|DestroyComponent (Variables|Default|GetProjectileEffect))
            (Utilities|FlowControl|Delay 2.0)
            (Actor|DestroyActor)))))))

(event EventTick
  (params (DeltaSeconds :type Float%20%28single-precision%29))
  (bind _projectileeffect (Variables|Default|GetProjectileEffect))
  ;[1 1 1] Update position and send it to the particle
  (if (Utilities|IsValid _projectileeffect)
    (Effects|Components|ParticleSystem|SetVectorParameter _projectileeffect "User.Position" (Transformation|GetActorLocation))))

(event EventBeginPlay
  (bind _explosion (Variables|Default|GetExplosion))
  (bind _projectileeffect (Variables|Default|GetProjectileEffect))
  (bind _sphere (Variables|Default|GetSphere))
  ;[1 1 1] Initialization
  (if (Variables|Default|GetbGravity)
    (Physics|SetEnableGravity _sphere true)
    (else
      (Physics|SetEnableGravity _sphere false)))
  (Physics|AddImpulse (Variables|Default|GetSphere) (* (Math|Vector|Normalize (Variables|Default|GetImpulseDirection)) (Variables|Default|GetImpulsePower)) "None" true)
  (Effects|Components|ParticleSystem|SetColorParameter _projectileeffect "User.Color" (Variables|Default|GetColor))
  (Effects|Components|ParticleSystem|SetFloatParameter _projectileeffect "User.Size" (Variables|Default|GetSize))
  (Effects|Components|ParticleSystem|SetColorParameter _explosion "User.Color" (Variables|Default|GetColor))
  (Effects|Components|ParticleSystem|SetFloatParameter _explosion "User.Size" (Variables|Default|GetSize)))

(fn ConstructionScript
  (bind _explosion (Variables|Default|GetExplosion))
  (bind _projectileeffect (Variables|Default|GetProjectileEffect))
  (switch int (Variables|Default|GetLevel)
    (:Default
      (Class|NiagaraComponent|SetAsset _projectileeffect "/Game/ThirdParty/Stylized_VFX_StPack/Particles/P_Classic_Projectile_03.P_Classic_Projectile_03" true :!label _label)
      (Class|NiagaraComponent|SetAsset _explosion "/Game/ThirdParty/Stylized_VFX_StPack/Particles/P_ExplosionEffect_03.P_ExplosionEffect_03" true))
    (:1
      (Class|NiagaraComponent|SetAsset _projectileeffect "/Game/ThirdParty/Stylized_VFX_StPack/Particles/P_Classic_Projectile_01.P_Classic_Projectile_01" true)
      (Class|NiagaraComponent|SetAsset _explosion "/Game/ThirdParty/Stylized_VFX_StPack/Particles/P_ExplosionEffect_01.P_ExplosionEffect_01" true))
    (:2
      (Class|NiagaraComponent|SetAsset _projectileeffect "/Game/ThirdParty/Stylized_VFX_StPack/Particles/P_Classic_Projectile_02.P_Classic_Projectile_02" true)
      (Class|NiagaraComponent|SetAsset _explosion "/Game/ThirdParty/Stylized_VFX_StPack/Particles/P_ExplosionEffect_02.P_ExplosionEffect_02" true))
    (:3
      (goto _label))))