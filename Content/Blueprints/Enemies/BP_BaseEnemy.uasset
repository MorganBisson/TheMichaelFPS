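; Base enemy Blueprint that handles life, damage, death and whether it can reach the player.
; After a short startup delay it registers with BP_MainGameMode and compares its nav mesh to the player's, binding to nav mesh overlap events.
; Projectile damage comes through RadialDamage and other damage through AnyDamage, both feeding UpdateLife.
; Death detaches the controller, disables capsule collision and tick, unregisters the enemy and applies any death material.
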(event Custom|DeathEvent
  (bind _deathmaterial (Variables|Default|GetDeathMaterial))
  ;[1 0 0.008376] Death
  (Variables|Default|SetisDead true)
  (Class|Pawn|DetachfromControllerPendingDestroy)
  (Collision|SetCollisionEnabled (Variables|Collision|GetCapsuleComponent) "NoCollision")
  (Actor|Tick|SetActorTickEnabled false)
  (bind _asbp_main_game_mode (Utilities|Casting|CastToBP_MainGameMode (Game|GetGameMode)))
  (Default|UnregisterEnemy _asbp_main_game_mode self)
  (Utilities|IsValid _deathmaterial
    (:Is%20Valid
      (Rendering|Material|SetMaterial (Variables|Character|GetMesh) 0 _deathmaterial))))

(event Custom|Event_CanReachThePlayer
  (bind _playerref (Variables|Default|GetPlayerRef))
  ;[1 1 1] Init data
  (if (and (Utilities|IsValid (Variables|Default|GetcurrentNavMesh)) (Utilities|IsValid _playerref))
    (if (== (Variables|Default|GetcurrentNavMesh) (Variables|/Game/FirstPersonBP/Blueprints/FirstPersonCharacter.FirstPersonCharacter_C|GetCurrentNavMesh _playerref))
      (Variables|Default|SetcanReachThePlayer true)
      (else
        (Variables|Default|SetcanReachThePlayer false)))))

(event EventUpdateLife
  (params (ValueToAdd :type Float%20%28single-precision%29))
  (bind _ac_lifealteration (Variables|Default|GetAC_LifeAlteration))
  ;[0.1599 0.7576 1] Update Life (interface)
  (bind _output_get (Variables|Default|SetLife (Math|Float|Clamp(Float) (+ ValueToAdd (Variables|Default|GetLife)) 0.0 (Variables|Default|GetMaxLife))))
  (if (<= _output_get 0.0)
    (CallFunction|DeathEvent))
  (Utilities|IsValid _ac_lifealteration
    (:Is%20Valid
      (Default|UpdateRenderingwhenAlive _ac_lifealteration))))

(event EventBeginPlay
  ;[1 1 1] Init data
  (Utilities|FlowControl|Delay 0.2) ; At least, doing this init step after the Game Mode is initialized
  (Utilities|FlowControl|Sequence
    (:then_0
      (Variables|Default|SetLife (Variables|Default|GetMaxLife))
      (if (not (Variables|Default|GetwillMove))
        (Variables|Default|SetAIControllerClass 0)))
    (:then_1
      (bind _asbp_main_game_mode (Utilities|Casting|CastToBP_MainGameMode (Game|GetGameMode)))
      (Default|RegisterEnemy _asbp_main_game_mode self)
      (Variables|Default|SetPlayerRef (Variables|/Game/Blueprints/BP_MainGameMode.BP_MainGameMode_C|GetPlayer _asbp_main_game_mode))
      (EventDispatchers|BindEventtoOnPlayerIsOverlappingNewNavMesh _asbp_main_game_mode (delegate Custom|Event_CanReachThePlayer)))
    (:then_2
      (CallFunction|EventCanReachthePlayer))))

(event Game|Damage|EventAnyDamage
  (params (Damage :type Float%20%28single-precision%29) (DamageType :type Damage%20Type%20Object%20Reference) (InstigatedBy :type Controller%20Object%20Reference) (DamageCauser :type Actor%20Object%20Reference))
  ;[1 1 1] Events receive damages
  ;;[1 1 1] Works but to review
  (Utilities|Casting|CastToFirstPersonProjectile DamageCauser
    (:CastFailed
      (CallFunction|UpdateLife (* Damage -1.0)))))

(event Game|Damage|EventRadialDamage
  (params (DamageReceived :type Float%20%28single-precision%29) (DamageType :type Damage%20Type%20Object%20Reference) (Origin :type Vector :default "0, 0, 0") (HitInfo :type Hit%20Result%20Structure%20%28by%20ref%29) (InstigatedBy :type Controller%20Object%20Reference) (DamageCauser :type Actor%20Object%20Reference))
  ;[1 1 1] Events receive damages
  (bind _asfirst_person_projectile (Utilities|Casting|CastToFirstPersonProjectile DamageCauser))
  (CallFunction|UpdateLife (* (Variables|/Game/FirstPersonBP/Blueprints/FirstPersonProjectile.FirstPersonProjectile_C|GetDamageLife _asfirst_person_projectile) -1.0)))

(fn ConstructionScript)