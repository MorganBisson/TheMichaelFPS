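; BP_PlayerShield is a player shield that loses protection points when hit by enemy projectiles.
; Activate restores full points, visibility and collision through Reset, or hides the mesh and disables its collision.
; Hits from actors tagged EnemyProjectile, excluding the BP_BaseEnemy class, subtract fixed damage and deactivate the shield at zero.
; A dynamic material instance created on BeginPlay is meant for hit feedback, currently a placeholder parameter marked TO DO.
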(event OnComponentHit(SM_Shield)
  (params (HitComponent :type Primitive%20Component%20Object%20Reference) (OtherActor :type Actor%20Object%20Reference) (OtherComp :type Primitive%20Component%20Object%20Reference) (NormalImpulse :type Vector :default "0, 0, 0") (Hit :type Hit%20Result%20Structure%20%28by%20ref%29))
  ;[1 1 1] Damages only received by the enemy projectiles
  (if (and (Actor|ActorHasTag OtherActor "EnemyProjectile") (!= (Utilities|GetClass OtherActor) "/Game/Blueprints/Enemies/BP_BaseEnemy.BP_BaseEnemy_C"))
    (bind _output_get (Variables|Default|SetCurrentProtectionPoints (- (Variables|Default|GetCurrentProtectionPoints) (Variables|Default|GetDamageReceivedPerProjectile))))
    (if (<= _output_get 0.0)
      (CallFunction|Activate false)
      (else
        ;[1 0.4169 0] TO DO
        (Rendering|Material|SetScalarParameterValue (Variables|Default|GetMI_Shield) "Demo" 0.0 :!class /Script/Engine.MaterialInstanceDynamic)))))

(event Custom|Reset
  (bind _sm_shield (Variables|Default|GetSM_Shield))
  ;[1 1 1] Reset state
  (Variables|Default|SetCurrentProtectionPoints (Variables|Default|GetDefaultProtectionPoints))
  (Collision|SetCollisionEnabled _sm_shield "QueryAndPhysics")
  (Rendering|SetVisibility _sm_shield true false))

(event Custom|Activate
  (params (NewState :type Boolean))
  (bind _sm_shield (Variables|Default|GetSM_Shield))
  ;[1 1 1] Enable / Disable shield
  (if NewState
    (CallFunction|Reset)
    (else
      (Collision|SetCollisionEnabled _sm_shield "NoCollision")
      (Rendering|SetVisibility _sm_shield false false))))

(event EventBeginPlay
  (bind _sm_shield (Variables|Default|GetSM_Shield))
  ;[1 1 1] Initialization
  (bind _returnvalue (Rendering|Material|CreateDynamicMaterialInstance _sm_shield 0 (Rendering|Material|GetMaterial _sm_shield 0) "None" :!class /Script/Engine.PrimitiveComponent))
  (Variables|Default|SetMI_Shield _returnvalue)
  (CallFunction|Reset))

(fn ConstructionScript)